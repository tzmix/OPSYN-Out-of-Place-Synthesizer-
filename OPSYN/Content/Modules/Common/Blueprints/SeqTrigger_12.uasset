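; Pressable trigger button for step 12 of an OSC-linked sequencer, with a glowing frame.
; Blocking overlaps depress the button, notify an optional ButtonActionInterface target, change four linked lights' colors and toggle the step via a counter, sending seqOn12/seqOff12 over OSC.
; Tick drives the frame's dynamic-material glow from local state and OSC.SeqLight12, brightest when both are on.
; Light_On/Light_Off events let a Euclidean source set the step without sending OSC.
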(event OnComponentBeginOverlap(Box)
  (params (OverlappedComponent :type Primitive%20Component%20Object%20Reference) (OtherActor :type Actor%20Object%20Reference) (OtherComp :type Primitive%20Component%20Object%20Reference) (OtherBodyIndex :type Integer) (bFromSweep :type Boolean) (SweepResult :type Hit%20Result%20Structure%20%28by%20ref%29))
  (bind _osc (Variables|Default|GetOSC))
  (bind _glow_material (Variables|Default|GetGlow%20Material))
  (if (Utilities|Enum|Equal(Enum) (Collision|GetCollisionResponsetoChannel OtherComp "ECC_PhysicsBody") "ECR_Block") ; only allow blockers to press
    (Variables|Default|SetPresser OtherActor)
    (CallFunction|PushDownButton)
    (Utilities|FlowControl|Sequence
      (:then_0
        (Default|ChangeLightColor (Variables|Default|GetLight%20Blueprint%201))
        (Default|ChangeLightColor (Variables|Default|GetLight%20Blueprint%202))
        (Default|ChangeLightColor (Variables|Default|GetLight%20Blueprint%203))
        (Default|ChangeLightColor (Variables|Default|GetLight%20Blueprint%204)))
      (:then_1
        (Variables|Default|SetLight true)
        (if (== (Variables|Default|GetConunter) 1)
          (Variables|Default|SetConunter 0)
          (Variables|Default|SetLight false)
          (else
            (bind _result (Math|Integer|IncrementInt (Variables|Default|GetConunter))
              (:%20%20
                (Variables|Default|SetConunter _result))))))
      (:then_2
        (if (Variables|Default|GetLight)
          (Utilities|FlowControl|Sequence
            (:then_0
              (Default|AddOSCMessage _osc "/seqOn12" (Class|OscFunctionLibrary|PushString 0 "seqOn")))
            (:then_1
              ;[1 1 1] Change Material Parameters
              (Rendering|Material|SetScalarParameterValue _glow_material "Edge Subtraction" -0.1 :!class /Script/Engine.MaterialInstanceDynamic)
              (if (Variables|/Game/OSC_BP.OSC_BP_C|GetSeqLight12 (Variables|Default|GetOSC))
                (if (Variables|Default|GetLight)
                  (Rendering|Material|SetScalarParameterValue _glow_material "Glow Strength" 2e+03 :!class /Script/Engine.MaterialInstanceDynamic)
                  (else
                    (Rendering|Material|SetScalarParameterValue _glow_material "Glow Strength" 1e+03 :!class /Script/Engine.MaterialInstanceDynamic :!label _label)))
                (else
                  (goto _label)))))
          (else
            (Utilities|FlowControl|Sequence
              (:then_0
                (Default|AddOSCMessage _osc "/seqOff12" (Class|OscFunctionLibrary|PushString 0 "seqOff")))
              (:then_1
                (Rendering|Material|SetScalarParameterValue _glow_material "Edge Subtraction" 0.1 :!class /Script/Engine.MaterialInstanceDynamic)
                (Rendering|Material|SetScalarParameterValue _glow_material "Glow Strength" 2.5e+02 :!class /Script/Engine.MaterialInstanceDynamic)))))))))

(event OnComponentEndOverlap(Box)
  (params (OverlappedComponent :type Primitive%20Component%20Object%20Reference) (OtherActor :type Actor%20Object%20Reference) (OtherComp :type Primitive%20Component%20Object%20Reference) (OtherBodyIndex :type Integer))
  (if (== OtherActor (Variables|Default|GetPresser))
    (Variables|Default|SetPresser 0)
    (CallFunction|ReleaseButton)))

(event Custom|Light_On
  (bind _glow_material (Variables|Default|GetGlow%20Material))
  ;[1 1 1] From Euclidean
  (Variables|Default|SetLight true)
  ;[1 1 1] Change Material Parameters
  (Rendering|Material|SetScalarParameterValue _glow_material "Edge Subtraction" -0.1 :!class /Script/Engine.MaterialInstanceDynamic)
  (if (Variables|/Game/OSC_BP.OSC_BP_C|GetSeqLight12 (Variables|Default|GetOSC))
    (if (Variables|Default|GetLight)
      (Rendering|Material|SetScalarParameterValue _glow_material "Glow Strength" 2e+03 :!class /Script/Engine.MaterialInstanceDynamic)
      (else
        (Rendering|Material|SetScalarParameterValue _glow_material "Glow Strength" 1e+03 :!class /Script/Engine.MaterialInstanceDynamic :!label _label)))
    (else
      (goto _label))))

(event Custom|Light_Off
  (bind _glow_material (Variables|Default|GetGlow%20Material))
  ;[1 1 1] From Euclidean
  (Variables|Default|SetLight false)
  ;[1 1 1] Change Material Parameters
  (Rendering|Material|SetScalarParameterValue _glow_material "Edge Subtraction" 0.1 :!class /Script/Engine.MaterialInstanceDynamic)
  (Rendering|Material|SetScalarParameterValue _glow_material "Glow Strength" 2.5e+02 :!class /Script/Engine.MaterialInstanceDynamic))

(event EventBeginPlay
  (bind _returnvalue (Rendering|Material|CreateDynamicMaterialInstance (Variables|Default|GetFrame) 0 0 "None" :!class /Script/Engine.PrimitiveComponent))
  (Variables|Default|SetGlow%20Material _returnvalue))

(event Collision|EventActorBeginOverlap
  (params (OtherActor :type Actor%20Object%20Reference)))

(event EventTick
  (params (DeltaSeconds :type Float%20%28single-precision%29))
  (bind _osc (Variables|Default|GetOSC))
  (bind _light (Variables|Default|GetLight))
  (bind _glow_material (Variables|Default|GetGlow%20Material))
  (bind _seqlight12 (Variables|/Game/OSC_BP.OSC_BP_C|GetSeqLight12 _osc))
  (if _seqlight12
    ;[1 1 1] Change Material Parameters
    (Rendering|Material|SetScalarParameterValue _glow_material "Edge Subtraction" -0.1 :!class /Script/Engine.MaterialInstanceDynamic :!label _label)
    (if _seqlight12
      (if _light
        (Rendering|Material|SetScalarParameterValue _glow_material "Glow Strength" 2e+03 :!class /Script/Engine.MaterialInstanceDynamic)
        (else
          (Rendering|Material|SetScalarParameterValue _glow_material "Glow Strength" 1e+03 :!class /Script/Engine.MaterialInstanceDynamic :!label _label_2)))
      (else
        (goto _label_2)))
    (elif _light
      (goto _label)
      (else
        (Rendering|Material|SetScalarParameterValue _glow_material "Edge Subtraction" 0.1 :!class /Script/Engine.MaterialInstanceDynamic)
        (Rendering|Material|SetScalarParameterValue _glow_material "Glow Strength" 2.5e+02 :!class /Script/Engine.MaterialInstanceDynamic)))))

(fn ConstructionScript
  (Variables|Default|SetDefaultButtonPosition (Variables|/Script/Engine.SceneComponent|GetRelativeLocation (Variables|Default|GetButton))))

(fn ReleaseButton
  (Transformation|SetRelativeLocation (Variables|Default|GetButton) (Variables|Default|GetDefaultButtonPosition) false false))

(fn PushDownButton
  (bind _actionlink (Variables|Default|GetActionLink))
  (Transformation|SetRelativeLocation (Variables|Default|GetButton) "0, 0, 0" false false)
  (if (!= _actionlink 0)
    (if (Utilities|DoesObjectImplementInterface _actionlink "/Game/Modules/Common/Blueprints/ButtonActionInterface.ButtonActionInterface_C")
      (Class|ButtonActionInterface|OnButtonPressed(Message) _actionlink)
      (else
        (Development|PrintString "Warning linked object doesn't implement  ButtonActionInterface")))))