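; Pressure-pad button Blueprint that sinks when a physics-blocking component overlaps its box and pops back when that presser leaves.
; Pressing notifies the linked actor through ButtonActionInterface, changes the color of four linked light Blueprints and raises the glow on a dynamic material.
; Press and release also send OSC messages on pad-5-specific addresses, while release restores the glow without reverting the lights or notifying the linked actor.
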(event OnComponentBeginOverlap(Box)
  (params (OverlappedComponent :type Primitive%20Component%20Object%20Reference) (OtherActor :type Actor%20Object%20Reference) (OtherComp :type Primitive%20Component%20Object%20Reference) (OtherBodyIndex :type Integer) (bFromSweep :type Boolean) (SweepResult :type Hit%20Result%20Structure%20%28by%20ref%29))
  (bind _glow_material (Variables|Default|GetGlow%20Material))
  (if (Utilities|Enum|Equal(Enum) (Collision|GetCollisionResponsetoChannel OtherComp "ECC_PhysicsBody") "ECR_Block") ; only allow blockers to press
    (Variables|Default|SetPresser OtherActor)
    (CallFunction|PushDownButton)
    (Default|AddOSCMessage (Variables|Default|GetOSC) "/padOn5" (Class|OscFunctionLibrary|PushString 0 "padOn"))
    (Default|ChangeLightColor (Variables|Default|GetLight%20Blueprint%201))
    (Default|ChangeLightColor (Variables|Default|GetLight%20Blueprint%202))
    (Default|ChangeLightColor (Variables|Default|GetLight%20Blueprint%203))
    (Default|ChangeLightColor (Variables|Default|GetLight%20Blueprint%204))
    ;[1 1 1] Change Material Parameters
    (Rendering|Material|SetScalarParameterValue _glow_material "Edge Subtraction" -0.1 :!class /Script/Engine.MaterialInstanceDynamic)
    (Rendering|Material|SetScalarParameterValue _glow_material "Glow Strength" 1e+03 :!class /Script/Engine.MaterialInstanceDynamic)))

(event OnComponentEndOverlap(Box)
  (params (OverlappedComponent :type Primitive%20Component%20Object%20Reference) (OtherActor :type Actor%20Object%20Reference) (OtherComp :type Primitive%20Component%20Object%20Reference) (OtherBodyIndex :type Integer))
  (bind _glow_material (Variables|Default|GetGlow%20Material))
  (if (== OtherActor (Variables|Default|GetPresser))
    (Variables|Default|SetPresser 0)
    (CallFunction|ReleaseButton)
    (Default|AddOSCMessage (Variables|Default|GetOSC) "/padOff5" (Class|OscFunctionLibrary|PushString 0 "padOff"))
    ;[1 1 1] Change Material Parameters
    (Rendering|Material|SetScalarParameterValue _glow_material "Edge Subtraction" 0.1 :!class /Script/Engine.MaterialInstanceDynamic)
    (Rendering|Material|SetScalarParameterValue _glow_material "Glow Strength" 2.5e+02 :!class /Script/Engine.MaterialInstanceDynamic)))

(event EventBeginPlay
  (bind _returnvalue (Rendering|Material|CreateDynamicMaterialInstance (Variables|Default|GetButton) 0 0 "None" :!class /Script/Engine.PrimitiveComponent))
  (Variables|Default|SetGlow%20Material _returnvalue))

(event Collision|EventActorBeginOverlap
  (params (OtherActor :type Actor%20Object%20Reference)))

(fn ConstructionScript
  (Variables|Default|SetDefaultButtonPosition (Variables|/Script/Engine.SceneComponent|GetRelativeLocation (Variables|Default|GetButton))))

(fn ReleaseButton
  (Transformation|SetRelativeLocation (Variables|Default|GetButton) (Variables|Default|GetDefaultButtonPosition) false false))

(fn PushDownButton
  (bind _actionlink (Variables|Default|GetActionLink))
  (Transformation|SetRelativeLocation (Variables|Default|GetButton) "0, 0, 0" false false)
  (if (!= _actionlink 0)
    (if (Utilities|DoesObjectImplementInterface _actionlink "/Game/Modules/Common/Blueprints/ButtonActionInterface.ButtonActionInterface_C")
      (Class|ButtonActionInterface|OnButtonPressed(Message) _actionlink)
      (else
        (Development|PrintString "Warning linked object doesn't implement  ButtonActionInterface")))))