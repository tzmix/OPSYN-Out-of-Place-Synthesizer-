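; ButtonTrigger7 is a pressure-pad actor that sinks when something overlaps its box and notifies a linked actor through ButtonActionInterface.
; Only components that block PhysicsBody can press it, and the button returns to its construction-time position when the stored presser leaves.
; Press and release also send OSC messages on addresses hardcoded for pad 7, while the linked actor is notified only on press.
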(event OnComponentBeginOverlap(Box)
  (params (OverlappedComponent :type Primitive%20Component%20Object%20Reference) (OtherActor :type Actor%20Object%20Reference) (OtherComp :type Primitive%20Component%20Object%20Reference) (OtherBodyIndex :type Integer) (bFromSweep :type Boolean) (SweepResult :type Hit%20Result%20Structure%20%28by%20ref%29))
  (if (Utilities|Enum|Equal(Enum) (Collision|GetCollisionResponsetoChannel OtherComp "ECC_PhysicsBody") "ECR_Block") ; only allow blockers to press
    (Variables|Default|SetPresser OtherActor)
    (CallFunction|PushDownButton)
    (Default|AddOSCMessage (Variables|Default|GetOSC) "/padOn7" (Class|OscFunctionLibrary|PushString 0 "padOn"))))

(event OnComponentEndOverlap(Box)
  (params (OverlappedComponent :type Primitive%20Component%20Object%20Reference) (OtherActor :type Actor%20Object%20Reference) (OtherComp :type Primitive%20Component%20Object%20Reference) (OtherBodyIndex :type Integer))
  (if (== OtherActor (Variables|Default|GetPresser))
    (Variables|Default|SetPresser 0)
    (CallFunction|ReleaseButton)
    (Default|AddOSCMessage (Variables|Default|GetOSC) "/padOff7" (Class|OscFunctionLibrary|PushString 0 "padOff"))))

(event EventBeginPlay)

(event Collision|EventActorBeginOverlap
  (params (OtherActor :type Actor%20Object%20Reference)))

(fn ConstructionScript
  (Variables|Default|SetDefaultButtonPosition (Variables|/Script/Engine.SceneComponent|GetRelativeLocation (Variables|Default|GetButton))))

(fn ReleaseButton
  (Transformation|SetRelativeLocation (Variables|Default|GetButton) (Variables|Default|GetDefaultButtonPosition) false false))

(fn PushDownButton
  (bind _actionlink (Variables|Default|GetActionLink))
  (Transformation|SetRelativeLocation (Variables|Default|GetButton) "0, 0, 0" false false)
  (if (!= _actionlink 0)
    (if (Utilities|DoesObjectImplementInterface _actionlink "/Game/Modules/Common/Blueprints/ButtonActionInterface.ButtonActionInterface_C")
      (Class|ButtonActionInterface|OnButtonPressed(Message) _actionlink)
      (else
        (Development|PrintString "Warning linked object doesn't implement  ButtonActionInterface")))))