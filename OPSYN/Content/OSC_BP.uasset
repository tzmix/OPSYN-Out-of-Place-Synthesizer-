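; OSC_BP is a two-way Open Sound Control test bridge between the game and a remote controller.
; The first received message registers the sender as a send target and starts a looping timer; later messages only print debug text, with two multifader addresses recognized.
; Tick queues the player pawn's location and P queues a test label, which the timer flushes as one bundle.
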(event Custom|OSCRx
  (params (Address :type Name%20%28by%20ref%29) (Data :type Array%20of%20Osc%20Data%20Elem%20Struct%20Structures) (SenderIp :type String))
  (if (Variables|Default|GetOSC_Ticking)
    (switch string (Utilities|String|ToString(Name) Address)
      (:Default
        (Development|PrintString (Utilities|String|ToString(Text) (Utilities|Text|FormatText "OSC Rx from {ip} - address {add} - VALUE {val}" (Utilities|Text|ToText(String) SenderIp) (Utilities|Text|ToText(Name) Address) (Utilities|Text|ToText(Float) (.Value (Class|OscFunctionLibrary|PopFloat Data)) "HalfToEven")))))
      (:/1/multifader1/1
        (Development|PrintString "fader1"))
      (:/1/multifader1/2
        (Development|PrintString "fader2")))
    (else
      (Class|OscFunctionLibrary|AddSendOscTarget (Utilities|String|ToString(Text) (Utilities|Text|FormatText "{ip}: 8080" (Utilities|Text|ToText(String) SenderIp))))
      (CallFunction|StartOSCTimer)
      (Variables|Default|SetOSC_Ticking true))))

(event Custom|StartOSCTimer
  (Utilities|Time|SetTimerbyEvent (delegate Custom|OSC%20Ticker) 0.05 true)
  (Development|PrintString "Received Input - OSC Ticker Started"))

(event Custom|OSC%20Ticker
  (bind _oscmessages (Variables|Default|GetOscMessages))
  (if (> (Utilities|Array|Length _oscmessages) 0)
    (Class|OscFunctionLibrary|SendOscBundle _oscmessages -1)
    (Utilities|Array|Clear _oscmessages)
    (Development|PrintString "String Sent")))

(event Custom|AddOSCMessage
  (params (TargetAddress :type String) (OSCData :type Array%20of%20Osc%20Data%20Elem%20Struct%20Structures))
  (Utilities|Array|Add (Variables|Default|GetOscMessages) (Utilities|Struct|MakeOscMessageStruct (Utilities|String|StringToName TargetAddress) OSCData)))

(event EventBeginPlay
  (EventDispatchers|BindEventtoOnOscReceived (Variables|Default|GetOscReceiver) (delegate Custom|OSCRx))
  (Development|PrintString "BP STARTED"))

(event Collision|EventActorBeginOverlap
  (params (OtherActor :type Actor%20Object%20Reference)))

(event EventTick
  (params (DeltaSeconds :type Float%20%28single-precision%29))
  (bind _returnvalue (Game|Player|GetPlayerPawn 0))
  (bind _returnvalue_2 (Transformation|GetActorLocation _returnvalue))
  (bind (_x _y _z) (Math|Vector|BreakVector _returnvalue_2))
  (CallFunction|AddOSCMessage "/1/position" (Class|OscFunctionLibrary|PushFloat (Class|OscFunctionLibrary|PushFloat (Class|OscFunctionLibrary|PushFloat 0 _x) _y) _z)))

(event Input|KeyboardEvents|P
  (params (Key :type Key%20Structure))
  (:Pressed
    (CallFunction|AddOSCMessage "/1/MyLabel" (Class|OscFunctionLibrary|PushString 0 "Hello"))
    (Development|PrintString "Added Data")))

(fn ConstructionScript)